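; Checkpoint trigger actor that saves the player's position to, or clears it from, the "Check" save slot on overlap.
; When its Load flag is set, it records the ThirdPersonCharacter's location and writes it to a Save_Checkpoint object with Load true, creating the save if none exists.
; Otherwise, it sets the saved Load flag to false, so one Blueprint serves as either a save or clear point.
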(event `self.Trigger.OnComponentBeginOverlap`
  (params (OverlappedComponent :type "PrimitiveComponent Object Reference") (OtherActor :type "Actor Object Reference") (OtherComp :type "PrimitiveComponent Object Reference") (OtherBodyIndex :type Integer) (bFromSweep :type Boolean) (SweepResult :type "HitResult Structure (by ref)"))
  (bind _playerloc (`self.PlayerLoc`))
  (if (`self.Load?`)
    (`|ExecutionSequence`
      (:`then_0`
        ;[1 1 1] Set Player Location for Checkpoint
        (bind _asthird_person_character (cast `/Game/ThirdPersonBP/Blueprints/ThirdPersonCharacter` (`GameplayStatics.GetPlayerCharacter` 0)))
        (set `self.PlayerLoc` (`self.K2_GetActorLocation` _asthird_person_character))
        (`KismetSystemLibrary.PrintString` "Checpoint Reached"))
      (:`then_1`
        ;[1 1 1] Save Player Location for Checkpoint
        (bind _returnvalue (`GameplayStatics.DoesSaveGameExist` "Check"))
        (if _returnvalue
          (bind _returnvalue_2 (`GameplayStatics.LoadGameFromSlot` "Check"))
          (bind _assave_checkpoint (cast `/Game/Checkpoint/Save_Checkpoint` _returnvalue_2))
          (set `/Game/Checkpoint/Save_Checkpoint.Player Loc S` _playerloc _assave_checkpoint)
          (set `/Game/Checkpoint/Save_Checkpoint.Load?` true _assave_checkpoint)
          (`GameplayStatics.SaveGameToSlot` _assave_checkpoint "Check")
          (else
            (bind _returnvalue_3 (`GameplayStatics.CreateSaveGameObject` "/Game/Checkpoint/Save_Checkpoint.Save_Checkpoint_C"))
            (set `/Game/Checkpoint/Save_Checkpoint.Player Loc S` _playerloc _returnvalue_3)
            (set `/Game/Checkpoint/Save_Checkpoint.Load?` true _returnvalue_3)
            (`GameplayStatics.SaveGameToSlot` _returnvalue_3 "Check")))))
    (else
      ;[1 1 1] Clears saved location upon reaching
      (bind _returnvalue_4 (`GameplayStatics.LoadGameFromSlot` "Check"))
      (bind _assave_checkpoint_2 (cast `/Game/Checkpoint/Save_Checkpoint` _returnvalue_4))
      (set `/Game/Checkpoint/Save_Checkpoint.Load?` false _assave_checkpoint_2)
      (`GameplayStatics.SaveGameToSlot` _assave_checkpoint_2 "Check")
      (`KismetSystemLibrary.PrintString` "Checkpoint Cleared"))))

(fn `UserConstructionScript`)